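; Stealth-game enemy AI character that patrols, chases the player on sight and investigates thrown distractions.
; Tick drives AI MoveTo, either looping through target points or picking random reachable points, with a CanMove flag enforcing pauses between moves.
; PawnSensing sight triggers a faster chase that overrides CanMove, and a retriggerable delay clears visibility when sightings stop.
; Hearing a distraction item sends the enemy walking to its path end to linger.
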(event `self.ReceiveBeginPlay`)

(event `self.ReceiveTick`
  (params (DeltaSeconds :type "Float (single-precision)"))
  (bind _bplayervisible (`self.bPlayerVisible`))
  (if (`self.bCanMove`)
    (if _bplayervisible
      (`self.ChasePlayer`)
      (elif (`self.TargetPointMovement`)
        (`self.MoveToNextPatrolPoint`)
        (else
          (`self.PatrolRandom`)
          (`KismetSystemLibrary.PrintString` "using random point"))))
    (elif _bplayervisible
      (`self.ChasePlayer`))))

(event `self.PawnSensing.OnSeePawn`
  (params (Pawn :type "Pawn Object Reference"))
  (`|ExecutionSequence`
    (:`then_0`
      (cast `/Game/StealthGame/Core/Characters/PlayerCharacter/BP_ThirdPersonCharacterCustom` Pawn
        (:`then`
          (`KismetSystemLibrary.PrintString` "Hey! Stop right there!")
          (set `self.bPlayerVisible` true))
        (:`CastFailed`
          (set `self.bPlayerVisible` false))))
    (:`then_1`
      (`KismetSystemLibrary.RetriggerableDelay` 1.0)
      (`KismetSystemLibrary.PrintString` "Must have been the wind...")
      (set `self.bPlayerVisible` false))))

(event `ChasePlayer`
  (`KismetSystemLibrary.PrintString` "CHASE PLAYER ACTIVATED")
  (`self.UpdateWalkSpeed` 600.0)
  (set `self.bCanMove` false)
  (`|AIMoveTo` self (0.0 0.0 0.0) (`GameplayStatics.GetPlayerCharacter` 0) 80.0
    (:`OnSuccess`
      _)
    (:`OnFail`
      _))
  (`KismetSystemLibrary.Delay` 3.0)
  (set `self.bCanMove` true))

(event `PatrolRandom`
  (`KismetSystemLibrary.PrintString` "PATROL RANDOM ACTIVATED")
  (`self.UpdateWalkSpeed` 200.0)
  (set `self.bCanMove` false)
  (`|AIMoveTo` self (`NavigationSystemV1.K2_GetRandomReachablePointInRadius` (`self.K2_GetActorLocation`) 2000.0 null null) null 80.0
    (:`OnSuccess`
      (`KismetSystemLibrary.Delay` 3.0)
      (set `self.bCanMove` true))))

(event `MoveToNextPatrolPoint`
  (`KismetSystemLibrary.PrintString` "MOVE TO NEXT PATROL POINT ACTIVATED")
  (`self.UpdateWalkSpeed` 200.0)
  (set `self.bCanMove` false)
  (`|AIMoveTo` self (0.0 0.0 0.0) (`|GetArrayItem` (`self.PatrolTargetPoints`) (`self.PatrolTargetPointIndex`)) 80.0
    (:`OnSuccess`
      (`KismetSystemLibrary.Delay` 3.0)
      (set `self.bCanMove` true)
      (`self.SetNextPatrolPointIndex`))))

(event `SetNextPatrolPointIndex`
  (set `self.PatrolTargetPointIndex` (mod (+ (`self.PatrolTargetPointIndex`) 1) (`KismetArrayLibrary.Array_Length` (`self.PatrolTargetPoints`)))))

(event `self.PawnSensing.OnHearNoise`
  (params (Instigator :type "Pawn Object Reference") (Location :type "Vector Structure (by ref)") (Volume :type "Float (single-precision)"))
  (bind _asbp_distraction_item_pawn (cast `/Game/StealthGame/Gadgets/NoiseMakers/BP_DistractionItemPawn` Instigator))
  (`self.UpdateWalkSpeed` 200.0)
  (set `self.bCanMove` false)
  (`|AIMoveTo` self (`/Game/StealthGame/Gadgets/NoiseMakers/BP_DistractionItemPawn.PathEndLocation` _asbp_distraction_item_pawn) null 80.0
    (:`OnSuccess`
      _)
    (:`OnFail`
      _))
  (`KismetSystemLibrary.Delay` 6.0) ; Rock distraction amount
  (set `self.bCanMove` true))

(fn `UpdateWalkSpeed`
  (params (NewWalkSpeed :type "Float (double-precision)"))
  (set `CharacterMovementComponent.MaxWalkSpeed` NewWalkSpeed (`self.CharacterMovement`)))

(fn `UserConstructionScript`)